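; Mod loader for FF7R that discovers, instantiates and drives Blueprint mods through lifecycle events.
; PreInit scans the Asset Registry for mod object, mod actor and extension classes, then LoadAllMods loads extensions before mods, checking plugin dependencies over capped recursive retries.
; Mod objects are constructed immediately, while actors spawn by SpawnTiming at PostInit or PostGameInstanceInit.
; Export objects then wrap each mod's config, metadata and active state.
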(event Custom|DelayUntilNextTickEvent
  (params (CallbackObject :type BPI%20Mod%20Objects%20Interface) (CallbackIndex :type Integer))
  (CallFunction|PrinttoModLoader (Utilities|String|Append "[" (Utilities|GetDisplayName (Utilities|ToObject(Interface) CallbackObject)) "]:" "End Delay Callback Index: " (Utilities|String|ToString(Integer) CallbackIndex)))
  (Default|DelayUntilNextTickCallback CallbackObject CallbackIndex))

(event EventPrinttoModLoader
  (params (Message :type String))
  (CallFunction|LogPrinttoModLoaderImpl Message self))

(event EventInit
  (CallFunction|PrinttoModLoader "Init")
  (CallFunction|CallDispatcher "NewEnumerator6")
  (CallFunction|CallDispatcher "NewEnumerator2"))

(event EventPostInit
  (CallFunction|PrinttoModLoader "PostInit")
  (CallFunction|SpawnModActors "NewEnumerator0")
  (CallFunction|CallDispatcher "NewEnumerator3"))

(event EventPreInit
  (if (Variables|Default|GetbLoggingEnabled)
    (bind _newdebugwidget (CallFunction|ConstructDebugWidget "" "FF7R ModLoader"))
    (Variables|Default|SetDebugWidget _newdebugwidget))
  (Variables|Default|SetCurrentLogDate (Math|DateTime|Now))
  (CallFunction|PrinttoModLoader "PreInit")
  (if (Variables|Default|GetbExtensionsEnabled)
    (for _array_element (Variables|Default|GetDefaultExtensionClasses)
      (CallFunction|LoadExtensions _array_element)))
  (bind _outassetdata (Class|AssetRegistry|GetAssets (Class|AssetRegistryHelpers|GetAssetRegistry) (Utilities|MakeARFilter 0 0 0 (Utilities|Array|MakeArray "Blueprint"))))
  (for _array_element_2 _outassetdata
    (bind _returnvalue (Utilities|LoadClassAssetBlocking (Class|KismetSystemLibrary|ToSoftClassRef(SoftClassPath) (Class|KismetSystemLibrary|MakeSoftClassPath (Utilities|String|Append (Utilities|String|ToString(Name) (.PackageName (Utilities|Struct|BreakAssetData _array_element_2))) "." (Utilities|String|ToString(Name) (.AssetName (Utilities|Struct|BreakAssetData _array_element_2))) "_C")))))
    (Utilities|Casting|CastToBP_ModObjectClass _returnvalue
      (:then
        _)
      (:CastFailed
        (Utilities|Casting|CastToBP_ModActorClass _returnvalue
          (:then
            _)
          (:CastFailed
            (Utilities|Casting|CastToBP_FF7RModLoaderExtension_BaseClass _returnvalue)))))
    (Utilities|Array|Add (Variables|Default|GetOutAssetData) _array_element_2))
  (CallFunction|LoadAllMods))

(event EventPostGameInstanceInit
  (CallFunction|PrinttoModLoader "PostGameStateInit")
  (CallFunction|SpawnModActors "NewEnumerator1")
  (CallFunction|CreateModExports)
  (CallFunction|CallDispatcher "NewEnumerator4"))

(event EventShutdown
  (for _array_element (Variables|Default|GetModObjects)
    (Default|Shutdown _array_element)))

(fn LoggingPrints
  (params (Message :type String))
  (if (Variables|Default|GetbLoggingEnabled)
    (Development|PrintString Message)
    (CallFunction|PrinttoDebugWidget "ModLoader" Message false)))

(fn LogPrinttoModLoaderImpl
  (params (Message :type String) (This :type Object%20Object%20Reference))
  (CallFunction|LoggingPrints (Utilities|String|Append "{" (Utilities|String|ToString(Name) (CallFunction|GetModNamefromPath (Utilities|ToString(SoftClassReference) (Utilities|ResolveSoftReference (Utilities|GetClass This))))) "}" Message)))

(fn CallDispatcher
  (params (InDelegate :type UDE_Dispatchers%20Enum :default "NewEnumerator0"))
  (switch Utilities|FlowControl|Switch|SwitchonUDE_Dispatchers InDelegate
    (:NewEnumerator0
      (for _array_element (Variables|Default|GetFF7RLoadedSubObjects)
        (bind _output_get (LocalVariables|SetCurrentObject _array_element))
        (if (Utilities|DoesObjectImplementInterface _output_get "/FF7RML/Interfaces/BPI_Mods.BPI_Mods_C")
          (Class|BPIMods|BindEvents(Message) (LocalVariables|GetCurrentObject)))))
    (:NewEnumerator1
      (Default|CallPreInitDispatch))
    (:NewEnumerator2
      (Default|CallInitDispatch))
    (:NewEnumerator3
      (Default|CallPostInitDispatch))
    (:NewEnumerator4
      (Default|CallPostGameInstanceInitDispatch))
    (:NewEnumerator5
      (Default|CallShutdownDispatch))
    (:NewEnumerator6
      (Default|CallLoadDataDispatch))))

(fn SpawnModActors
  (params (InTiming :type UDE_SpawnTiming%20Enum :default "NewEnumerator0"))
  (for _array_element (Variables|Default|GetModActorClasses)
    (if (== (.SpawnTiming (Utilities|GetClassDefaults _array_element)) InTiming)
      (bind _asend_game_instance (Utilities|Casting|CastToEndGameInstance (Game|GetGameInstance)))
      (bind _returnvalue (Game|SpawnActorfromClass _array_element (Math|Transform|MakeTransform "0, 0, 0" "0, 0, 0" "1,1,1") "Undefined" 0 true 0 _asend_game_instance self 0))
      (Utilities|Array|AddUnique (Variables|Default|GetModActors) _returnvalue)
      (Class|BPIMods|BindEvents(Message) _returnvalue)))
  (return))

(fn SpawnActor
  (params (Class :type Actor%20Class%20Reference) (SpawnTransform :type Transform) (CollisionHandlingOverride :type ESpawnActorCollisionHandlingMethod%20Enum :default "Undefined") (Owner :type Actor%20Object%20Reference) (Instigator :type Pawn%20Object%20Reference))
  (bind _returnvalue (Game|SpawnActorfromClass Class SpawnTransform CollisionHandlingOverride Owner Instigator))
  (return _returnvalue))

(fn LoadAllMods
  (bind _self self)
  (bind _ff7rloadedsubobjects (Variables|Default|GetFF7RLoadedSubObjects))
  (bind _result (Math|Integer|IncrementInt (Variables|Default|GetModLoadLoops))
    (:%20%20
      (if (<= _result 3)
        (bind (_arrayindex _arrayelement) (Utilities|Array|ReverseforEachLoop (Variables|Default|GetOutAssetData))
          (:LoopBody
            (LocalVariables|SetCurrentAssetData _arrayelement)
            (LocalVariables|SetCurrentAssetDataIndex _arrayindex)
            (if (Utilities|String|Contains (Utilities|String|ToString(Name) (.PackagePath (Utilities|Struct|BreakAssetData (LocalVariables|GetCurrentAssetData)))) "FF7RML") :!label _label
              (Utilities|Array|RemoveIndex (Variables|Default|GetOutAssetData) (LocalVariables|GetCurrentAssetDataIndex))
              (else
                (CallFunction|PrinttoModLoader (Utilities|String|Append (Utilities|String|ToString(Name) (.PackageName (Utilities|Struct|BreakAssetData (LocalVariables|GetCurrentAssetData)))) "." (Utilities|String|ToString(Name) (.AssetName (Utilities|Struct|BreakAssetData (LocalVariables|GetCurrentAssetData)))) "_C"))
                (bind _da_metadata (CallFunction|GetMetaDataDA (CallFunction|GetModNamefromPath (Utilities|String|ToString(Name) (.PackagePath (Utilities|Struct|BreakAssetData (LocalVariables|GetCurrentAssetData)))))))
                (Utilities|Map|Add (Variables|Default|GetModMetaData) (CallFunction|GetModNamefromPath (Utilities|String|ToString(Name) (.PackagePath (Utilities|Struct|BreakAssetData (LocalVariables|GetCurrentAssetData))))) _da_metadata)
                (if (> (Utilities|Array|Length (.Plugins (Utilities|Struct|BreakUDS_ModMetaData _da_metadata))) 0)
                  (bind _array_element (Utilities|Array|ForEachLoopwithBreak (.Plugins (Utilities|Struct|BreakUDS_ModMetaData _da_metadata)) :!label _label_2)
                    (:LoopBody
                      (if (Utilities|Name|Equal(Name) (.name _array_element) "FF7RML")
                        (LocalVariables|SetbFoundDeps (Utilities|Name|Equal(Name) (.name _array_element) "FF7RML"))
                        (else
                          (bind _output_get (LocalVariables|SetbFoundDeps (.ReturnValue (Utilities|Map|Find (Variables|Default|GetModMetaData) (.name _array_element)))))
                          (if (not _output_get)
                            (goto _label_2 Break)))))
                    (:Completed
                      (if (LocalVariables|GetbFoundDeps)
                        (bind _da_metadata_2 (CallFunction|GetModConfigDA (CallFunction|GetModNamefromPath (Utilities|String|ToString(Name) (.PackagePath (Utilities|Struct|BreakAssetData (LocalVariables|GetCurrentAssetData))))) :!label _label_3))
                        (Utilities|Map|Add (Variables|Default|GetModConfig) (CallFunction|GetModNamefromPath (Utilities|String|ToString(Name) (.PackagePath (Utilities|Struct|BreakAssetData (LocalVariables|GetCurrentAssetData))))) _da_metadata_2)
                        (bind _returnvalue (Utilities|LoadClassAssetBlocking (Class|KismetSystemLibrary|ToSoftClassRef(SoftClassPath) (Class|KismetSystemLibrary|MakeSoftClassPath (Utilities|String|Append (Utilities|String|ToString(Name) (.PackageName (Utilities|Struct|BreakAssetData (LocalVariables|GetCurrentAssetData)))) "." (Utilities|String|ToString(Name) (.AssetName (Utilities|Struct|BreakAssetData (LocalVariables|GetCurrentAssetData)))) "_C")))))
                        (if (LocalVariables|GetbExtensionsLoaded)
                          (bind _asbp_mod_object (Utilities|Casting|CastToBP_ModObjectClass _returnvalue)
                            (:then
                              (bind _asend_game_instance (Utilities|Casting|CastToEndGameInstance (Game|GetGameInstance)))
                              (bind _returnvalue_2 (Game|ConstructObjectfromClass _asbp_mod_object _self _asend_game_instance _self))
                              (Utilities|Array|Add (Variables|Default|GetModObjects) _returnvalue_2)
                              (Utilities|Array|RemoveIndex (Variables|Default|GetOutAssetData) (LocalVariables|GetCurrentAssetDataIndex)))
                            (:CastFailed
                              (bind _asbp_mod_actor (Utilities|Casting|CastToBP_ModActorClass _returnvalue))
                              (Utilities|Array|AddUnique (Variables|Default|GetModActorClasses) _asbp_mod_actor)
                              (Utilities|Array|RemoveIndex (Variables|Default|GetOutAssetData) (LocalVariables|GetCurrentAssetDataIndex))))
                          (else
                            (bind _asbp_ff7rmod_loader_extension_base (Utilities|Casting|CastToBP_FF7RModLoaderExtension_BaseClass _returnvalue))
                            (CallFunction|LoadExtensions _asbp_ff7rmod_loader_extension_base)
                            (Utilities|Array|RemoveIndex (Variables|Default|GetOutAssetData) (LocalVariables|GetCurrentAssetDataIndex)))))))
                  (else
                    (goto _label_3))))))
          (:Completed
            (LocalVariables|SetbExtensionsLoaded true)
            (bind (_arrayindex_2 _arrayelement_2) (Utilities|Array|ReverseforEachLoop (Variables|Default|GetOutAssetData))
              (:LoopBody
                (LocalVariables|SetCurrentAssetData _arrayelement_2)
                (LocalVariables|SetCurrentAssetDataIndex _arrayindex_2)
                (goto _label))
              (:Completed
                (if (> (Utilities|Array|Length (Variables|Default|GetOutAssetData)) 0)
                  (CallFunction|LoadAllMods)
                  (else
                    (LocalVariables|SetCurrentAssetData "")
                    (LocalVariables|SetCurrentAssetDataIndex 0)
                    (Utilities|Array|AppendArray _ff7rloadedsubobjects (Variables|Default|GetExtensions))
                    (Utilities|Array|AppendArray _ff7rloadedsubobjects (Variables|Default|GetModObjects))
                    (CallFunction|CallDispatcher "NewEnumerator0")
                    (CallFunction|CallDispatcher "NewEnumerator1")))))))
        (else
          (Utilities|Array|Clear (Variables|Default|GetOutAssetData)))))))

(fn GetModUPlugin
  (params (ModName :type Name))
  (return ""))

(fn LoadExtensions
  (params (Class :type BP%20FF7R%20Mod%20Loader%20Extension%20Base%20Class%20Reference))
  (bind _self self)
  (bind _asbp_ff7rmod_loader_extension_base (Utilities|Casting|CastToBP_FF7RModLoaderExtension_BaseClass Class))
  (bind _returnvalue (Game|ConstructObjectfromClass _asbp_ff7rmod_loader_extension_base _self _self))
  (CallFunction|PrinttoModLoader (Utilities|String|Append "Extension Loaded: " (Utilities|GetDisplayName _returnvalue)))
  (Default|BindEvents _returnvalue)
  (Utilities|Array|AddUnique (Variables|Default|GetExtensions) _returnvalue)
  (return))

(fn CreateModExports
  (for _array_element (Variables|Default|GetModObjects)
    (bind _asbpi_mods (Utilities|Casting|CastToBPI_Mods _array_element))
    (bind _returnvalue (Game|ConstructObjectfromClass "/FF7RML/Classes/BP_ModExport.BP_ModExport_C" self (Variables|/FF7RML/Classes/BP_ModObject.BP_ModObject_C|GetHasSettings _array_element) _asbpi_mods (.Value (Utilities|Map|Find (Variables|Default|GetModConfig) (CallFunction|GetModNamefromPath (Utilities|ToString(SoftClassReference) (Utilities|ResolveSoftReference (Utilities|GetClass _array_element)))))) (.Value (Utilities|Map|Find (Variables|Default|GetModMetaData) (CallFunction|GetModNamefromPath (Utilities|ToString(SoftClassReference) (Utilities|ResolveSoftReference (Utilities|GetClass _array_element)))))) self (CallFunction|GetModNamefromPath (Utilities|ToString(SoftClassReference) (Utilities|ResolveSoftReference (Utilities|GetClass _array_element))))))
    (bind _deactivated (Default|IsDeactivated _asbpi_mods))
    (Variables|/FF7RML/Classes/BP_ModExport.BP_ModExport_C|SetIsActive _returnvalue (not _deactivated))
    (Utilities|Array|AddUnique (Variables|Default|GetModExports) _returnvalue))
  (for _array_element_2 (Variables|Default|GetModActors)
    (Variables|/FF7RML/Classes/BP_ModActor.BP_ModActor_C|SetModName _array_element_2 (CallFunction|GetModNamefromPath (Utilities|ToString(SoftClassReference) (Utilities|ResolveSoftReference (Utilities|GetClass _array_element_2)))))
    (bind _asbpi_mods_2 (Utilities|Casting|CastToBPI_Mods _array_element_2))
    (bind _returnvalue_2 (Game|ConstructObjectfromClass "/FF7RML/Classes/BP_ModExport.BP_ModExport_C" self (Variables|/FF7RML/Classes/BP_ModActor.BP_ModActor_C|GetHasSettings _array_element_2) _asbpi_mods_2 (.Value (Utilities|Map|Find (Variables|Default|GetModConfig) (CallFunction|GetModNamefromPath (Utilities|ToString(SoftClassReference) (Utilities|ResolveSoftReference (Utilities|GetClass _array_element_2)))))) (.Value (Utilities|Map|Find (Variables|Default|GetModMetaData) (CallFunction|GetModNamefromPath (Utilities|ToString(SoftClassReference) (Utilities|ResolveSoftReference (Utilities|GetClass _array_element_2)))))) self (CallFunction|GetModNamefromPath (Utilities|ToString(SoftClassReference) (Utilities|ResolveSoftReference (Utilities|GetClass _array_element_2))))))
    (Default|LoadData _returnvalue_2)
    (bind _deactivated_2 (Default|IsDeactivated _asbpi_mods_2))
    (Variables|/FF7RML/Classes/BP_ModExport.BP_ModExport_C|SetIsActive _returnvalue_2 (not _deactivated_2))
    (Utilities|Array|AddUnique (Variables|Default|GetModExports) _returnvalue_2)))

(fn CreateWidget
  (params (Class :type User%20Widget%20Class%20Reference) (OwningPlayer :type Player%20Controller%20Object%20Reference))
  (bind _returnvalue (UserInterface|CreateWidget Class OwningPlayer))
  (return _returnvalue))

(fn GetModExports
  (return (Variables|Default|GetModExports)))

(fn PrintAssetRegistry
  (bind _outassetdata (Class|AssetRegistry|GetAllAssets (Class|AssetRegistryHelpers|GetAssetRegistry) false))
  (for _array_element _outassetdata
    (if (Utilities|String|Contains (Utilities|GetClassDisplayName (Class|AssetRegistryHelpers|GetClass _array_element)) "BP_ModObject")
      (Class|EndMenuAPI|AddMessageLogAnyThread "None" (Utilities|GetClassDisplayName (Class|AssetRegistryHelpers|GetClass _array_element)) "None" "Default" "None")))
  (Class|EndMenuAPI|AddMessageLogAnyThread "None" (Utilities|String|Append (Utilities|String|ToString(Integer) (Utilities|Array|Length _outassetdata)) " Assets found") "None" "Default" "None"))

(fn GetModConfigDA
  (params (ModName :type Name))
  (bind _returnvalue (Utilities|LoadAssetBlocking (Class|KismetSystemLibrary|ToSoftObjRef(SoftObjPath) (Utilities|MakeSoftObjectPath (Utilities|String|Append "/" (Utilities|String|ToString(Name) ModName) "/" "MetaData/" "DA_ModConfig.DA_ModConfig")))))
  (bind _aspda_mod_config (Utilities|Casting|CastToPDA_ModConfig _returnvalue))
  (return _aspda_mod_config))

(fn DelayUntilNextTickImpl
  (params (CallbackObject :type BPI%20Mod%20Objects%20Interface))
  (bind _returnvalue (Utilities|Array|Add (Variables|Default|GetDelayCallbacks) CallbackObject))
  (CallFunction|DelayUntilNextTickEvent CallbackObject _returnvalue)
  (return _returnvalue))

(fn GetAllInstalledMods
  (bind _keys (Utilities|Map|Keys (Variables|Default|GetModMetaData)))
  (return _keys))