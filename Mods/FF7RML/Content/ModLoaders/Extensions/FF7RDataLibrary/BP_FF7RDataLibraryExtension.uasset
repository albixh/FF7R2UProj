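; FF7R mod loader extension that builds a data library of installed mods from their data assets.
; On PreInit it scans the Asset Registry outside FF7RML paths, blocking-loads each mod asset and sorts it by ModType into maps keyed by mod name.
; It also stores metadata and registers a BP_ModExport per mod with the loader.
; A SaveGame filter persists deactivated mods, with functions to remove or re-add their map entries.
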(event EventPreInit
  (CallFunction|LoadFilter)
  (CallFunction|LoadModDas))

(event EventInit)

(fn LoadModDas
  (bind _outassetdata (Class|AssetRegistry|GetAssets (Class|AssetRegistryHelpers|GetAssetRegistry) (Utilities|MakeARFilter 0 0 0 (Utilities|Array|MakeArray "DataAsset") 0 false true)))
  (for _array_element _outassetdata
    (if (not (Utilities|String|Contains (Utilities|String|ToString(Name) (.PackagePath (Utilities|Struct|BreakAssetData _array_element))) "FF7RML"))
      (bind _returnvalue (Utilities|LoadAssetBlocking (Class|KismetSystemLibrary|ToSoftObjRef(SoftObjPath) (Utilities|MakeSoftObjectPath (Utilities|String|Append (Utilities|String|ToString(Name) (.PackageName (Utilities|Struct|BreakAssetData _array_element))) "." (Utilities|String|ToString(Name) (.AssetName (Utilities|Struct|BreakAssetData _array_element))))))))
      (bind _aspda_mod_data_base (Utilities|Casting|CastToPDA_ModData_Base _returnvalue))
      (CallFunction|PrinttoModLoader (Utilities|String|Append "Found Mod DA:" (Utilities|String|Append (Utilities|String|ToString(Name) (.PackageName (Utilities|Struct|BreakAssetData _array_element))) "." (Utilities|String|ToString(Name) (.AssetName (Utilities|Struct|BreakAssetData _array_element))))))
      (Utilities|Array|Add (Variables|Default|GetModData) _array_element)
      (Utilities|FlowControl|Sequence
        (:then_0
          (switch Utilities|FlowControl|Switch|SwitchonE_ModType (Variables|/FF7RML/ModLoaders/Extensions/FF7RDataLibrary/Structs/PDA_ModData_Base.PDA_ModData_Base_C|GetMod%20Type _aspda_mod_data_base)
            (:NewEnumerator0
              (bind _aspda_mod_data_object (Utilities|Casting|CastToPDA_ModData_Object _aspda_mod_data_base))
              (Utilities|Map|Add (Variables|Default|GetObjectData) (CallFunction|GetModNamefromPath (Utilities|String|ToString(Name) (.PackagePath (Utilities|Struct|BreakAssetData _array_element)))) _aspda_mod_data_object))
            (:NewEnumerator5
              (bind _aspda_mod_data_texture (Utilities|Casting|CastToPDA_ModData_Texture _aspda_mod_data_base))
              (Utilities|Map|Add (Variables|Default|GetTextureData) (CallFunction|GetModNamefromPath (Utilities|String|ToString(Name) (.PackagePath (Utilities|Struct|BreakAssetData _array_element)))) _aspda_mod_data_texture))
            (:NewEnumerator7
              (bind _aspda_mod_data_material (Utilities|Casting|CastToPDA_ModData_Material _aspda_mod_data_base))
              (Utilities|Map|Add (Variables|Default|GetMaterialData) (CallFunction|GetModNamefromPath (Utilities|String|ToString(Name) (.PackagePath (Utilities|Struct|BreakAssetData _array_element)))) _aspda_mod_data_material))
            (:NewEnumerator1
              (bind _aspda_mod_data_character (Utilities|Casting|CastToPDA_ModData_Character _aspda_mod_data_base))
              (Utilities|Map|Add (Variables|Default|GetHairData) (CallFunction|GetModNamefromPath (Utilities|String|ToString(Name) (.PackagePath (Utilities|Struct|BreakAssetData _array_element)))) _aspda_mod_data_character))
            (:NewEnumerator2
              (bind _aspda_mod_data_character_2 (Utilities|Casting|CastToPDA_ModData_Character _aspda_mod_data_base))
              (Utilities|Map|Add (Variables|Default|GetWeaponData) (CallFunction|GetModNamefromPath (Utilities|String|ToString(Name) (.PackagePath (Utilities|Struct|BreakAssetData _array_element)))) _aspda_mod_data_character_2))
            (:NewEnumerator3
              (bind _aspda_mod_data_character_3 (Utilities|Casting|CastToPDA_ModData_Character _aspda_mod_data_base))
              (Utilities|Map|Add (Variables|Default|GetCharacterData) (CallFunction|GetModNamefromPath (Utilities|String|ToString(Name) (.PackagePath (Utilities|Struct|BreakAssetData _array_element)))) _aspda_mod_data_character_3))
            (:NewEnumerator8
              (bind _aspda_mod_data_character_4 (Utilities|Casting|CastToPDA_ModData_Character _aspda_mod_data_base))
              (Utilities|Map|Add (Variables|Default|GetVehicleData) (CallFunction|GetModNamefromPath (Utilities|String|ToString(Name) (.PackagePath (Utilities|Struct|BreakAssetData _array_element)))) _aspda_mod_data_character_4))
            (:NewEnumerator6
              (bind _aspda_mod_data_level (Utilities|Casting|CastToPDA_ModData_Level _aspda_mod_data_base))
              (Utilities|Map|Add (Variables|Default|GetLevelData) (CallFunction|GetModNamefromPath (Utilities|String|ToString(Name) (.PackagePath (Utilities|Struct|BreakAssetData _array_element)))) _aspda_mod_data_level))))
        (:then_1
          (bind _da_metadata (CallFunction|GetMetaDataDA (CallFunction|GetModNamefromPath (Utilities|String|ToString(Name) (.PackagePath (Utilities|Struct|BreakAssetData _array_element))))))
          (Utilities|Map|Add (Variables|Default|GetModMetaData) (CallFunction|GetModNamefromPath (Utilities|String|ToString(Name) (.PackagePath (Utilities|Struct|BreakAssetData _array_element)))) _da_metadata)
          (bind _returnvalue_2 (Game|ConstructObjectfromClass "/FF7RML/Classes/BP_ModExport.BP_ModExport_C" self false 0 0 _da_metadata (CallFunction|GetModLoader) (CallFunction|GetModNamefromPath (Utilities|String|ToString(Name) (.PackagePath (Utilities|Struct|BreakAssetData _array_element))))))
          (Variables|/FF7RML/Classes/BP_ModExport.BP_ModExport_C|SetIsActive _returnvalue_2 (not (Utilities|Array|ContainsItem (Variables|/FF7RML/ModLoaders/Extensions/FF7RDataLibrary/BP_FF7RDataLibraryFilter.BP_FF7RDataLibraryFilter_C|GetDeactivatedMods (Variables|Default|GetBP_Filter)) (Variables|/FF7RML/Classes/BP_ModExport.BP_ModExport_C|GetModName _returnvalue_2))))
          (Utilities|Array|AddUnique (Variables|/FF7RML/ModLoaders/BP_FF7RModLoader.BP_FF7RModLoader_C|GetExtensionModExports (CallFunction|GetModLoader)) _returnvalue_2)))))
  (for _array_element_2 (Variables|/FF7RML/ModLoaders/Extensions/FF7RDataLibrary/BP_FF7RDataLibraryFilter.BP_FF7RDataLibraryFilter_C|GetDeactivatedMods (Variables|Default|GetBP_Filter))
    (CallFunction|FilterModData _array_element_2)))

(fn FilterModData
  (params (ModName :type Name%20%28by%20ref%29))
  (Utilities|Map|Remove (Variables|Default|GetModMetaData) ModName)
  (Utilities|Map|Remove (Variables|Default|GetCharacterData) ModName)
  (Utilities|Map|Remove (Variables|Default|GetHairData) ModName)
  (Utilities|Map|Remove (Variables|Default|GetVehicleData) ModName)
  (Utilities|Map|Remove (Variables|Default|GetWeaponData) ModName)
  (Utilities|Map|Remove (Variables|Default|GetTextureData) ModName)
  (Utilities|Map|Remove (Variables|Default|GetMaterialData) ModName)
  (Utilities|Map|Remove (Variables|Default|GetLevelData) ModName)
  (Utilities|Map|Remove (Variables|Default|GetAudioData) ModName))

(fn DeactivateModData
  (params (ModName :type Name%20%28by%20ref%29))
  (Utilities|Array|AddUnique (Variables|/FF7RML/ModLoaders/Extensions/FF7RDataLibrary/BP_FF7RDataLibraryFilter.BP_FF7RDataLibraryFilter_C|GetDeactivatedMods (Variables|Default|GetBP_Filter)) ModName)
  (CallFunction|FilterModData ModName)
  (CallFunction|SaveFilter))

(fn ActivateModData
  (params (ModName :type Name%20%28by%20ref%29))
  (Utilities|Array|RemoveItem (Variables|/FF7RML/ModLoaders/Extensions/FF7RDataLibrary/BP_FF7RDataLibraryFilter.BP_FF7RDataLibraryFilter_C|GetDeactivatedMods (Variables|Default|GetBP_Filter)) ModName)
  (CallFunction|SaveFilter)
  (for _array_element (Variables|Default|GetModData)
    (if (Utilities|String|Contains (Utilities|String|ToString(Name) (.PackagePath (Utilities|Struct|BreakAssetData _array_element))) (Utilities|String|ToString(Name) ModName))
      (bind _returnvalue (Utilities|LoadAssetBlocking (Class|KismetSystemLibrary|ToSoftObjRef(SoftObjPath) (Utilities|MakeSoftObjectPath (Utilities|String|Append (Utilities|String|ToString(Name) (.PackageName (Utilities|Struct|BreakAssetData _array_element))) "." (Utilities|String|ToString(Name) (.AssetName (Utilities|Struct|BreakAssetData _array_element))))))))
      (bind _aspda_mod_data_base (Utilities|Casting|CastToPDA_ModData_Base _returnvalue))
      (Utilities|FlowControl|Sequence
        (:then_0
          (switch Utilities|FlowControl|Switch|SwitchonE_ModType (Variables|/FF7RML/ModLoaders/Extensions/FF7RDataLibrary/Structs/PDA_ModData_Base.PDA_ModData_Base_C|GetMod%20Type _aspda_mod_data_base)
            (:NewEnumerator5
              (bind _aspda_mod_data_texture (Utilities|Casting|CastToPDA_ModData_Texture _aspda_mod_data_base))
              (Utilities|Map|Add (Variables|Default|GetTextureData) "" _aspda_mod_data_texture))
            (:NewEnumerator7
              (bind _aspda_mod_data_material (Utilities|Casting|CastToPDA_ModData_Material _aspda_mod_data_base))
              (Utilities|Map|Add (Variables|Default|GetMaterialData) "" _aspda_mod_data_material))
            (:NewEnumerator1
              (bind _aspda_mod_data_character (Utilities|Casting|CastToPDA_ModData_Character _aspda_mod_data_base))
              (Utilities|Map|Add (Variables|Default|GetHairData) "" _aspda_mod_data_character))
            (:NewEnumerator2
              (bind _aspda_mod_data_character_2 (Utilities|Casting|CastToPDA_ModData_Character _aspda_mod_data_base))
              (Utilities|Map|Add (Variables|Default|GetWeaponData) "" _aspda_mod_data_character_2))
            (:NewEnumerator3
              (bind _aspda_mod_data_character_3 (Utilities|Casting|CastToPDA_ModData_Character _aspda_mod_data_base))
              (Utilities|Map|Add (Variables|Default|GetCharacterData) "" _aspda_mod_data_character_3))
            (:NewEnumerator8
              (bind _aspda_mod_data_character_4 (Utilities|Casting|CastToPDA_ModData_Character _aspda_mod_data_base))
              (Utilities|Map|Add (Variables|Default|GetVehicleData) "" _aspda_mod_data_character_4))
            (:NewEnumerator6
              (bind _aspda_mod_data_level (Utilities|Casting|CastToPDA_ModData_Level _aspda_mod_data_base))
              (Utilities|Map|Add (Variables|Default|GetLevelData) "" _aspda_mod_data_level))))))))

(fn LoadFilter
  (bind _returnvalue (SaveGame|LoadGamefromSlot (Utilities|String|Append "FF7RDataLibrary_Filter" "")))
  (bind _asbp_ff7rdata_library_filter (Utilities|Casting|CastToBP_FF7RDataLibraryFilter _returnvalue)
    (:then
      (Variables|Default|SetBP_Filter _asbp_ff7rdata_library_filter))
    (:CastFailed
      (bind _returnvalue_2 (SaveGame|CreateSaveGameObject "/FF7RML/ModLoaders/Extensions/FF7RDataLibrary/BP_FF7RDataLibraryFilter.BP_FF7RDataLibraryFilter_C"))
      (Variables|Default|SetBP_Filter _returnvalue_2))))

(fn SaveFilter
  (Utilities|IsValid (Variables|Default|GetBP_Filter)
    (:Is%20Valid
      (SaveGame|SaveGametoSlot (Variables|Default|GetBP_Filter) (Utilities|String|Append "FF7RDataLibrary_Filter" "")))))