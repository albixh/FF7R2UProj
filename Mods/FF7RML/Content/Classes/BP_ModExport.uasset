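; BP_ModExport wraps one mod for the mod loader, handling its saved settings and its activation state.
; Settings save to a per-mod "ModConfig_" slot; loading merges only keys still present in the loader's config, then copies the result to the mod object or actor.
; Activation and shutdown go to that object or actor, or otherwise to the loader's FF7R data library extensions by mod name.
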(fn SaveData
  (params (InSave :type BP%20Mod%20Save%20Game%20Object%20Reference))
  (if (Variables|Default|GetHasSettings)
    (SaveGame|SaveGametoSlot InSave (Utilities|String|Append "ModConfig_" (Utilities|String|ToString(Name) (Variables|Default|GetModName))))
    (CallFunction|LoadData)))

(fn LoadData
  (bind _modname (Variables|Default|GetModName))
  (bind _modloader (Variables|Default|GetModLoader))
  (bind _modconfig (Variables|/FF7RML/ModLoaders/BP_FF7RModLoader.BP_FF7RModLoader_C|GetModConfig _modloader))
  (bind _value (Utilities|Map|Find _modconfig _modname))
  (bind _modconfiguration (Variables|/FF7RML/ModLoaders/Structs/PDA_ModConfig.PDA_ModConfig_C|GetModConfiguration _value))
  (Default|LoadData (Variables|Default|GetModObject))
  (if (Variables|Default|GetHasSettings)
    (bind _returnvalue (SaveGame|LoadGamefromSlot (Utilities|String|Append "ModConfig_" (Utilities|String|ToString(Name) (Variables|Default|GetModName)))))
    (bind _asbp_mod_save_game (Utilities|Casting|CastToBP_ModSaveGame _returnvalue))
    (bind _keys (Utilities|Map|Keys (Variables|/FF7RML/Classes/BP_ModSaveGame.BP_ModSaveGame_C|GetModConfigSaveData _asbp_mod_save_game)))
    (for _array_element _keys
      (if (.ReturnValue (Utilities|Map|Find _modconfiguration _array_element))
        (Utilities|Map|Add (Variables|/FF7RML/ModLoaders/Structs/PDA_ModConfig.PDA_ModConfig_C|GetModConfiguration (Variables|Default|GetModConfig)) _array_element (.Value (Utilities|Map|Find (Variables|/FF7RML/Classes/BP_ModSaveGame.BP_ModSaveGame_C|GetModConfigSaveData _asbp_mod_save_game) _array_element)))
        (Utilities|Map|Add _modconfiguration _array_element (.Value (Utilities|Map|Find (Variables|/FF7RML/Classes/BP_ModSaveGame.BP_ModSaveGame_C|GetModConfigSaveData _asbp_mod_save_game) _array_element)))))
    (CallFunction|UpdateModObject)))

(fn UpdateModObject
  (bind _asbp_mod_actor (Utilities|Casting|CastToBP_ModActor (Variables|Default|GetModObject))
    (:then
      (Variables|/FF7RML/Classes/BP_ModActor.BP_ModActor_C|SetModConfig _asbp_mod_actor (Variables|Default|GetModConfig)))
    (:CastFailed
      (bind _asbp_mod_object (Utilities|Casting|CastToBP_ModObject (Variables|Default|GetModObject)))
      (Variables|/FF7RML/Classes/BP_ModObject.BP_ModObject_C|SetModConfig _asbp_mod_object (Variables|Default|GetModConfig)))))

(fn ActivateMod
  (bind _modobject (Variables|Default|GetModObject))
  (bind _modobject_2 (Variables|Default|GetModObject))
  (Utilities|Casting|CastToBP_ModObject _modobject
    (:then
      (Default|Activate _modobject_2 :!label _label)
      (bind _deactivated (Default|IsDeactivated _modobject_2))
      (Variables|Default|SetIsActive (not _deactivated)))
    (:CastFailed
      (Utilities|Casting|CastToBP_ModActor _modobject
        (:then
          (goto _label))
        (:CastFailed
          (for _array_element (Variables|/FF7RML/ModLoaders/BP_FF7RModLoader.BP_FF7RModLoader_C|GetExtensions (Variables|Default|GetModLoader))
            (bind _asbp_ff7rdata_library_extension (Utilities|Casting|CastToBP_FF7RDataLibraryExtension _array_element))
            (Default|ActivateModData _asbp_ff7rdata_library_extension (Variables|Default|GetModName))
            (Variables|Default|SetIsActive true)))))))

(fn DeactivateMod
  (bind _modobject (Variables|Default|GetModObject))
  (bind _modobject_2 (Variables|Default|GetModObject))
  (Variables|Default|SetIsActive false)
  (Utilities|Casting|CastToBP_ModObject _modobject
    (:then
      (Default|Shutdown _modobject_2 :!label _label)
      (bind _deactivated (Default|IsDeactivated _modobject_2))
      (Variables|Default|SetIsActive (not _deactivated)))
    (:CastFailed
      (Utilities|Casting|CastToBP_ModActor _modobject
        (:then
          (goto _label))
        (:CastFailed
          (for _array_element (Variables|/FF7RML/ModLoaders/BP_FF7RModLoader.BP_FF7RModLoader_C|GetExtensions (Variables|Default|GetModLoader))
            (bind _asbp_ff7rdata_library_extension (Utilities|Casting|CastToBP_FF7RDataLibraryExtension _array_element))
            (Default|DeactivateModData _asbp_ff7rdata_library_extension (Variables|Default|GetModName))
            (Variables|Default|SetIsActive false)))))))